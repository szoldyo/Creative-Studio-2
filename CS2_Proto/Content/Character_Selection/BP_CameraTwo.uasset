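; BP_CameraTwo is the character selection camera for the second player, turning to face one of eight characters spaced 45 degrees apart.
; On BeginPlay it adds WBP_CharacterSelectTwo for player controller 1 and focuses it in Game and UI input mode.
; RotateCamera plays a Timeline that blends actor yaw from its current value toward the indexed angle.
; The gamepad bottom face button also nudges the Camera component's local rotation.
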(event `self.ReceiveBeginPlay`
  (bind _returnvalue (`GameplayStatics.GetPlayerController` 1))
  (bind _returnvalue_2 (`|CreateWidget` "/Game/UI/WBP_CharacterSelectTwo.WBP_CharacterSelectTwo_C" _returnvalue))
  (`UserWidget.AddToViewport` _returnvalue_2 0)
  (`WidgetBlueprintLibrary.SetInputMode_GameAndUIEx` _returnvalue _returnvalue_2))

(event `Key|Gamepad_FaceButton_Bottom`
  (params (Key :type "Key Structure"))
  (:`Pressed`
    (`SceneComponent.K2_AddLocalRotation` (`self.Camera`) (struct :`Yaw` 10.0) false false)))

(event `Rotate Camera`
  (params (Index :type Integer))
  (bind (_returnvalue_roll _returnvalue_pitch _returnvalue_yaw) (`KismetMathLibrary.BreakRotator` (`self.K2_GetActorRotation`)))
  (bind (_direction _newtrack_0) (`Timeline|Timeline` :!via `PlayFromStart`)
    (:`Update`
      (`self.K2_SetActorRotation` (`KismetMathLibrary.MakeRotator` 0.0 0.0 (`KismetMathLibrary.MapRangeClamped` _newtrack_0 0.0 1.0 _returnvalue_yaw (select `int` Index :`0` 0.0 :`1` 45.0 :`2` 90.0 :`3` 135.0 :`4` 180.0 :`5` -135.0 :`6` -90.0 :`7` -45.0)))))))

(fn `UserConstructionScript`)