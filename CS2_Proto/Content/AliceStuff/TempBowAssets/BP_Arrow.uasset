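; BP_Arrow is an arrow projectile actor that flies once fired from a detached state.
; Fire adds a projectile movement component at runtime, sets its velocity along the given direction at a fixed speed, then orients the arrow from player 0's BP_RangedClass rotation with roll and yaw offsets.
; Overlapping a BP_Player_M only prints a hit message, with no damage applied.
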(event `Fire`
  (params (Direction :type "Vector Structure"))
  ;[1 0.4784 0.9843] Gives movement and velocity to the detached arrow
  (bind _returnvalue (`AddComponent|NODE_AddProjectileMovementComponent-0`))
  (set `MovementComponent.Velocity` (* Direction 2500.0) _returnvalue)
  (bind _asbp_ranged_class (cast `/Game/AliceStuff/RangedClass/BP_RangedClass` (`GameplayStatics.GetPlayerCharacter` 0)))
  (bind (_returnvalue_roll _returnvalue_pitch _returnvalue_yaw) (`KismetMathLibrary.BreakRotator` (`self.K2_GetActorRotation` _asbp_ranged_class)))
  (`self.K2_SetActorRotation` (`KismetMathLibrary.MakeRotator` (- _returnvalue_roll 90.0) 0.0 (- _returnvalue_yaw 90.0))))

(event `self.ReceiveActorBeginOverlap`
  (params (OtherActor :type "Actor Object Reference"))
  (cast `/Game/Player/Classes/Melee/BP_Player_M` OtherActor)
  (`KismetSystemLibrary.PrintString` "Arrow Hit"))

(fn `UserConstructionScript`)