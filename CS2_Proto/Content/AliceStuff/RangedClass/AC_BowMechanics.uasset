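; Bow mechanics component for BP_RangedClass that handles aiming and firing arrows.
; Aiming turns the character with controller rotation and spawns a BP_Arrow on a mesh socket; ending aim restores movement-oriented rotation.
; Firing detaches and offsets the arrow, launches it along the character's forward vector, then respawns one after a delay, with a DoOnce as cooldown.
; DestroyArrow, uncalled here, clears all BP_Arrow actors when the current reference is valid.
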(event `self.ReceiveBeginPlay`
  ;[1 0.4784 0.9843] Spawns bow in player's hand and quiver on the back
  (bind _asbp_ranged_class (cast `/Game/AliceStuff/RangedClass/BP_RangedClass` (`self.GetOwner`)))
  (set `self.CharacterRef` _asbp_ranged_class)
  (set `self.InitialRotationRate` (`CharacterMovementComponent.RotationRate` (`Character.CharacterMovement` (`self.CharacterRef`)))))

(event `AimBegin`
  (bind _charactermovement (`Character.CharacterMovement` (`self.CharacterRef`)))
  ;[1 0.4784 0.9843] Locks player rotation to camera while aiming, and spawns/despawns the arrow while aiming
  (set `self.IsAiming` true)
  (set `CharacterMovementComponent.bOrientRotationToMovement` false _charactermovement)
  (set `CharacterMovementComponent.bUseControllerDesiredRotation` true _charactermovement)
  (set `CharacterMovementComponent.RotationRate` (`self.AimRotationRate`) _charactermovement)
  (`self.Spawn arrow`))

(event `AimEnd`
  (bind _charactermovement (`Character.CharacterMovement` (`self.CharacterRef`)))
  ;[1 0.4784 0.9843] Locks player rotation to camera while aiming, and spawns/despawns the arrow while aiming
  (set `self.IsAiming` false)
  (set `CharacterMovementComponent.bOrientRotationToMovement` true _charactermovement)
  (set `CharacterMovementComponent.bUseControllerDesiredRotation` false _charactermovement)
  (set `CharacterMovementComponent.RotationRate` (`self.InitialRotationRate`) _charactermovement))

(event `FireArrowBegin`
  ;[1 0.4784 0.9843] Detaches arrow from mesh, sets rotation and triggers firing BP
  (`/Engine/EditorBlueprintResources/StandardMacros.DoOnce` false :!label _label
    (:`Completed`
      (bind _arrowref (`self.ArrowRef`)
        (:`then`
          (`Actor.K2_DetachFromActor` _arrowref "KeepWorld" "KeepWorld" "KeepWorld")
          (`Actor.K2_AddActorLocalOffset` _arrowref (-50.0 0.0 80.0) false false)
          (`/Game/AliceStuff/Bow_BPs/BP_Arrow.Fire` _arrowref (`SceneComponent.GetForwardVector` (`Actor.RootComponent` (`self.CharacterRef`))))
          (`KismetSystemLibrary.Delay` 1.5)
          (`self.Spawn arrow`)
          (goto _label :!via `Reset`))
        (:`else`)))))

(fn `Destroy arrow`
  (bind _outactors (`GameplayStatics.GetAllActorsOfClass` "/Game/AliceStuff/Bow_BPs/BP_Arrow.BP_Arrow_C"))
  (`self.ArrowRef`
    (:`then`
      (`Actor.K2_DestroyActor` _outactors))
    (:`else`)))

(fn `Spawn arrow`
  ;[1 0.4784 0.9843] Yippie
  (bind _returnvalue (`|SpawnActorFromClass` "/Game/AliceStuff/Bow_BPs/BP_Arrow.BP_Arrow_C" (`KismetMathLibrary.MakeTransform` (0.0 0.0 0.0)) "Undefined" "MultiplyWithRoot" null null))
  (bind _output_get (set `self.ArrowRef` _returnvalue))
  (`Actor.K2_AttachToComponent` _output_get (`Character.Mesh` (`self.CharacterRef`)) (`self.ArrowSocketName`) "KeepRelative" "KeepRelative" "KeepRelative" true))