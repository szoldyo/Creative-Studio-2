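; Melee player character Blueprint with prototype sword combo attacks and a test UI widget added on BeginPlay.
; Two combo versions coexist: IA_Attack alternates two slash montages, while IA_Combo steps through an Attacks array, gated by MovementAllowed and reset by a retriggerable delay.
; HitDetect sphere-traces at the right-hand socket to damage test dummies through a DoOnce.
; A debug-style key plays draw or sheathe montages based on WeaponEquipped.
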(event `self.ReceiveBeginPlay`
  (`parent.ReceiveBeginPlay`)
  ;[1 0 0] TEST UI
  (bind _returnvalue (`|CreateWidget` "/Game/Player/Testing/PlayerOne_UI.PlayerOne_UI_C" (`GameplayStatics.GetPlayerController` 0)))
  (`UserWidget.AddToViewport` _returnvalue 0))

(event `EnhancedInput|/Game/Player/Master/Input/Actions/IA_Attack`
  (params (ActionValue :type Boolean) (ElapsedSeconds :type "Float (double-precision)") (TriggeredSeconds :type "Float (double-precision)") (InputAction :type "InputAction Object Reference" :default "/Game/Player/Master/Input/Actions/IA_Attack.IA_Attack"))
  ;[1 0.2781 0.2781] Combat Combo Animations version 1
  (:`Triggered`
    (if (not (`self.Attacking?`))
      (set `self.Attacking?` true)
      (`|PlayMontage` (`self.Mesh`) (select `int` (`self.AttackCount`) :`0` "/Game/Animations/Combat/AM_SwordSlash1.AM_SwordSlash1" :`1` "/Game/Animations/Combat/AM_SwordSlash2.AM_SwordSlash2" :!type "AnimMontage Object Reference")
        (:`then`
          (`/Engine/EditorBlueprintResources/StandardMacros.IncrementInt` (`self.AttackCount`)))
        (:`OnCompleted`
          (set `self.AttackCount` 0 :!label _label))
        (:`OnInterrupted`
          (`KismetSystemLibrary.RetriggerableDelay` 2.0)
          (set `self.Attacking?` false)
          (goto _label))))))

(event `EnhancedInput|/Game/Player/Master/Input/Actions/IA_Combo`
  (params (ActionValue :type Boolean) (ElapsedSeconds :type "Float (double-precision)") (TriggeredSeconds :type "Float (double-precision)") (InputAction :type "InputAction Object Reference" :default "/Game/Player/Master/Input/Actions/IA_Combo.IA_Combo"))
  ;[1 0.174 0.174] Combo animations version 2
  (:`Started`
    (if (`self.MovementAllowed?`)
      (set `self.MovementAllowed?` false)
      (bind _animation (`self.Perform Combo`))
      (`self.PlayAnimMontage` _animation))))

(event `Reset Player Movement`
  ;[1 0.174 0.174] Combo animations version 2
  ;;[1 1 1] Allow Player to Move
  (set `self.MovementAllowed?` true))

(event `Reset Combo`
  ;[1 0.174 0.174] Combo animations version 2
  ;;[1 1 1] Increase or Reset Combo
  (set `self.AttackCombo` 0 :!label _label_2))

(event `Perform Attack`
  ;[1 0.174 0.174] Combo animations version 2
  ;;[1 1 1] Increase or Reset Combo
  (`/Engine/EditorBlueprintResources/StandardMacros.IncrementInt` (`self.AttackCombo`)
    (:`  `
      (`KismetSystemLibrary.RetriggerableDelay` 2.0)
      (goto _label_2))))

(event `Key|One`
  (params (Key :type "Key Structure"))
  ;[1 0.9853 0] DO I EVEN USE IT?!?!?
  (:`Pressed`
    (if (`self.WeaponEquipped?`)
      (`self.PlayAnimMontage` "/Game/Animations/Combat/AM_SheatheSword.AM_SheatheSword")
      (else
        (`self.PlayAnimMontage` "/Game/Animations/Combat/AM_DrawSword.AM_DrawSword")))))

(fn `HitDetect`
  (bind _returnvalue (`SceneComponent.GetSocketLocation` (`self.Mesh`) "hand_r"))
  (bind _outhit (`KismetSystemLibrary.SphereTraceSingleForObjects` :`Start` _returnvalue :`End` _returnvalue :`Radius` 50.0 :`ObjectTypes` (`|MakeArray` "ObjectTypeQuery3" :!type "EObjectTypeQuery Enum") :`DrawDebugType` "ForDuration"))
  (bind _asbp_player_test_dummy (cast `/Game/Player/Classes/TestDummy/BP_PlayerTestDummy` (`.HitActor` (`GameplayStatics.BreakHitResult` _outhit))))
  (`/Engine/EditorBlueprintResources/StandardMacros.DoOnce` false
    (:`Completed`
      (`/Game/Player/Classes/TestDummy/BP_PlayerTestDummy.DamageTaken` _asbp_player_test_dummy))))

(fn `Perform Combo`
  (returns (Animation :type "AnimMontage Object Reference"))
  (bind _attacks (`self.Attacks`))
  (if (>= (`self.AttackCombo`) (- (`KismetArrayLibrary.Array_Length` (`self.Attacks`)) 1))
    (`self.Reset Combo`)
    (return (`|GetArrayItem` _attacks (`KismetArrayLibrary.Array_LastIndex` _attacks)))
    (else
      (`self.Perform Attack`)
      (return (`|GetArrayItem` (`self.Attacks`) (- (`self.AttackCombo`) 1))))))

(fn `UserConstructionScript`
  (`parent.UserConstructionScript`))