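; Test dummy player Blueprint that receives hits and can block, and creates the player-two UI for the second player controller on BeginPlay.
; DamageTaken ignores hits while blocking or already reacting, otherwise playing a hit montage and deducting fixed damage once, guarded by a DoOnce that resets when the montage ends.
; The mesh switches to physics simulation when health reaches exactly zero.
; IA_Block input holds the blocking flag while active.
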(event `self.ReceiveBeginPlay`
  (`parent.ReceiveBeginPlay`)
  ;[1 0 0] TEST UI
  (bind _returnvalue (`|CreateWidget` "/Game/UI/PlayerTwo_UI.PlayerTwo_UI_C" (`GameplayStatics.GetPlayerController` 1)))
  (`UserWidget.AddToViewport` _returnvalue 0))

(event `DamageTaken`
  (bind _health (`self.Health`))
  ;[1 0.2948 0.2948] Take Damage
  (if (`self.IsBlocking?`)
    _
    (elif (not (`self.GettingHit?`))
      (set `self.GettingHit?` true)
      (`|PlayMontage` (`self.Mesh`) "/Game/Animations/Combat/AM_Hit.AM_Hit" 1.5
        (:`then`
          (if (>= _health 0.0)
            (`/Engine/EditorBlueprintResources/StandardMacros.DoOnce` false :!label _label
              (:`Completed`
                (set `self.Health` (- _health 10.0))
                (if (== (`self.Health`) 0.0)
                  (`PrimitiveComponent.SetSimulatePhysics` (`self.Mesh`) true))))))
        (:`OnCompleted`
          (set `self.GettingHit?` false :!label _label_2)
          (goto _label :!via `Reset`))
        (:`OnInterrupted`
          (goto _label_2))))))

(event `EnhancedInput|/Game/Player/Master/Input/Actions/IA_Block`
  (params (ActionValue :type Boolean) (ElapsedSeconds :type "Float (double-precision)") (TriggeredSeconds :type "Float (double-precision)") (InputAction :type "InputAction Object Reference" :default "/Game/Player/Master/Input/Actions/IA_Block.IA_Block"))
  ;[0.9639 1 0] TESTING
  ;;[1 1 1] Basic Block
  (:`Triggered`
    (set `self.IsBlocking?` true :!label _label_3))
  (:`Ongoing`
    (goto _label_3))
  (:`Canceled`
    (set `self.IsBlocking?` false :!label _label_4))
  (:`Completed`
    (goto _label_4)))

(fn `UserConstructionScript`
  (`parent.UserConstructionScript`))